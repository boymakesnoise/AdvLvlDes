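; Player-controlled swimming turtle with a spring-arm orbit camera that eases toward body pitch and re-centres yaw on a button press.
; Tick moves it constantly forward along the Kroppen body component, with cooldown-limited strokes boosting a decaying speed.
; Axis input steers yaw and lerped pitch and roll.
; A downward trace forces a nose-up climb below a minimum height until a recovery height is reached; max-height logic is unconnected.
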(event `InputAxis|CameraUp`
  (params (AxisValue :type "Float (single-precision)"))
  (bind (_returnvalue_roll _returnvalue_pitch _returnvalue_yaw) (`KismetMathLibrary.BreakRotator` (`SceneComponent.K2_GetComponentRotation` (`self.SpringArm`))))
  ;[1 1 1] Camera
  (set `self.CamPitch` (`KismetMathLibrary.ClampAngle` (+ (/ AxisValue 2.0) _returnvalue_pitch) -70.0 30.0)))

(event `InputAxis|CameraRight`
  (params (AxisValue :type "Float (single-precision)"))
  (bind (_returnvalue_roll _returnvalue_pitch _returnvalue_yaw) (`KismetMathLibrary.BreakRotator` (`SceneComponent.K2_GetComponentRotation` (`self.SpringArm`))))
  ;[1 1 1] Camera
  (set `self.CamYaw` (+ (/ AxisValue 2.0) _returnvalue_yaw)))

(event `InputAxis|LookUp`
  (params (AxisValue :type "Float (single-precision)"))
  (bind _kroppen (`self.kroppen`))
  (bind (_relativerotation_roll _relativerotation_pitch _relativerotation_yaw) (`KismetMathLibrary.BreakRotator` (`SceneComponent.RelativeRotation` _kroppen)))
  ;[1 1 1] Steering
  (if (`self.IsAboveMinHeight`) :!label _label
    (`SceneComponent.K2_SetRelativeRotation` _kroppen (`KismetMathLibrary.MakeRotator` (`self.TurnAngle`) (`self.PitchAngle`) (+ (/ (stale `InputAxis|TurnRight` AxisValue) 8.0) _relativerotation_yaw)) false false)))

(event `InputAxis|TurnRight`
  (params (AxisValue :type "Float (single-precision)"))
  ;[1 1 1] Steering
  (goto _label))

(event `InputAction|SwimStroke`
  (params (Key :type "Key Structure"))
  ;[1 1 1] Swim Stroke
  (:`Pressed`
    (if (`self.CanStrokeAgain`)
      (set `self.CurrentSwimSpeed` (`self.SwimSpeed`))
      (set `self.CanStrokeAgain` false)
      (`KismetSystemLibrary.Delay` (`self.StrokeDuration`))
      (set `self.CanStrokeAgain` true))))

(event `self.ReceiveTick`
  (params (DeltaSeconds :type "Float (single-precision)"))
  (bind _pitchangle (`self.PitchAngle`))
  (bind _kroppen (`self.kroppen`))
  (bind _camyaw (`self.CamYaw`))
  (bind _returnvalue (`SceneComponent.K2_GetComponentLocation` (`self.LineTraceStart`)))
  (bind (_relativerotation_roll _relativerotation_pitch _relativerotation_yaw) (`KismetMathLibrary.BreakRotator` (`SceneComponent.RelativeRotation` _kroppen)))
  (bind (_relativerotation_roll_2 _relativerotation_pitch_2 _relativerotation_yaw_2) (`KismetMathLibrary.BreakRotator` (`SceneComponent.RelativeRotation` (`self.kroppen`))))
  (bind (_returnvalue_roll _returnvalue_pitch _returnvalue_yaw) (`KismetMathLibrary.BreakRotator` (`KismetMathLibrary.RLerp` (`KismetMathLibrary.MakeRotator` 0.0 0.0 _camyaw) (`KismetMathLibrary.MakeRotator` 0.0 0.0 _relativerotation_yaw_2) 0.025 true)))
  ;[1 1 1] LERP Cam Pitch
  (set `self.CamPitch` (`KismetMathLibrary.Lerp` (`self.CamPitch`) (- _relativerotation_pitch_2 30.0) 0.01))
  ;[1 1 1] Reset Cam Yaw
  (if (`self.YawBack?`)
    (set `self.CamYaw` _returnvalue_yaw)
    (`|ExecutionSequence`
      (:`then_0`
        (`KismetSystemLibrary.Delay` 1.0)
        (set `self.YawBack?` false :!label _label_2))
      (:`then_1`
        (if (`KismetMathLibrary.NearlyEqual_FloatFloat` _relativerotation_yaw_2 _camyaw 3.0)
          (goto _label_2)
          (else
            _)))))
  (`SceneComponent.K2_SetRelativeRotation` (`self.SpringArm`) (`KismetMathLibrary.MakeRotator` 0.0 (`self.CamPitch`) (`self.CamYaw`)) false false)
  ;[1 1 1] Forward movement
  (bind _output_get (set `self.CurrentSwimSpeed` (`KismetMathLibrary.FClamp` (- (`self.CurrentSwimSpeed`) 0.025) 1.0 (`self.SwimSpeed`))))
  (`SceneComponent.K2_AddWorldOffset` (`self.DefaultSceneRoot`) (* (`SceneComponent.GetForwardVector` (`self.kroppen`)) _output_get) false false)
  ;[1 1 1] LERP Roll Angle
  (set `self.TurnAngle` (`KismetMathLibrary.Lerp` (`self.TurnAngle`) (* (`self.GetInputAxisValue`) 70.0) 0.007))
  ;[1 1 1] Ground Check
  (bind _outhit (`KismetSystemLibrary.LineTraceSingle` _returnvalue (- _returnvalue (0.0 0.0 10000.0)) "TraceTypeQuery1"))
  (set `self.HeightAboveGround` (.z (- (`SceneComponent.K2_GetComponentLocation` (`self.LineTraceStart`)) (`.Location` (`GameplayStatics.BreakHitResult` _outhit)))))
  ;[1 1 1] LERP Pitch Angle
  (if (`self.IsAboveMinHeight`)
    (set `self.PitchAngle` (`KismetMathLibrary.Lerp` _pitchangle (`KismetMathLibrary.ClampAngle` (+ _pitchangle (* (`self.GetInputAxisValue`) -25.0)) -55.0 55.0) 0.01))
    ;[1 1 1] Set Bools
    (if (< (`self.HeightAboveGround`) (`self.MinHeight`))
      (set `self.IsAboveMinHeight` false))
    (else
      ;[1 1 1] Height Restrictions Up & Down
      (bind _output_get_2 (set `self.PitchAngle` (`KismetMathLibrary.Lerp` (`self.PitchAngle`) 45.0 0.005)))
      (`SceneComponent.K2_SetRelativeRotation` _kroppen (`KismetMathLibrary.MakeRotator` (`self.TurnAngle`) _output_get_2 _relativerotation_yaw) false false)
      (if (> (`self.HeightAboveGround`) (`self.MinRecoveryHeight`))
        (set `self.IsAboveMinHeight` true)))))

(event `InputAction|ResetCamYaw`
  (params (Key :type "Key Structure"))
  ;[1 1 1] Reset Cam Yaw
  (:`Pressed`
    (set `self.YawBack?` true)))

(fn `UserConstructionScript`)