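; Player-controlled swimming turtle with an orbiting spring-arm camera that can ease back behind the mesh.
; Holding SwimStroke replays the stroke animation and adds speed, which decays through drag and moves the actor along the mesh's forward vector.
; Tick smooths steering pitch and roll with lerps and stretches the camera arm with speed.
; Line traces down, up, left and right steer it away from floor, roof and walls; dash triggering is unwired.
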(event `InputAxis|CameraUp`
  (params (AxisValue :type "Float (single-precision)"))
  (bind (_returnvalue_roll _returnvalue_pitch _returnvalue_yaw) (`KismetMathLibrary.BreakRotator` (`SceneComponent.K2_GetComponentRotation` (`self.SpringArm`))))
  ;[1 1 1] Camera
  (set `self.CamPitch` (`KismetMathLibrary.ClampAngle` (+ (/ AxisValue 2.0) _returnvalue_pitch) -70.0 30.0)))

(event `InputAxis|CameraRight`
  (params (AxisValue :type "Float (single-precision)"))
  (bind (_returnvalue_roll _returnvalue_pitch _returnvalue_yaw) (`KismetMathLibrary.BreakRotator` (`SceneComponent.K2_GetComponentRotation` (`self.SpringArm`))))
  ;[1 1 1] Camera
  (set `self.CamYaw` (+ (/ AxisValue 2.0) _returnvalue_yaw)))

(event `InputAxis|LookUp`
  (params (AxisValue :type "Float (single-precision)"))
  (bind _skeletalmesh (`self.SkeletalMesh`))
  (bind (_relativerotation_roll _relativerotation_pitch _relativerotation_yaw) (`KismetMathLibrary.BreakRotator` (`SceneComponent.RelativeRotation` _skeletalmesh)))
  ;[1 1 1] Steering
  (if (`self.IsAboveMinHeight`) :!label _label
    (`SceneComponent.K2_SetRelativeRotation` _skeletalmesh (`KismetMathLibrary.MakeRotator` (`self.TurnAngle`) (`self.PitchAngle`) (+ (/ (stale `InputAxis|TurnRight` AxisValue) 7.0) _relativerotation_yaw)) false false)))

(event `InputAxis|TurnRight`
  (params (AxisValue :type "Float (single-precision)"))
  ;[1 1 1] Steering
  (goto _label))

(event `InputAction|SwimStroke`
  (params (Key :type "Key Structure"))
  ;[1 1 1] Swim Stroke
  (:`Pressed`
    (set `self.Swimming?` true))
  (:`Released`
    (set `self.Swimming?` false)))

(event `InputAction|Dash`
  (params (Key :type "Key Structure"))
  ;[1 1 1] Dash
)

(event `self.ReceiveTick`
  (params (DeltaSeconds :type "Float (single-precision)"))
  (bind _pitchangle (`self.PitchAngle`))
  (bind _currentswimspeed (`self.CurrentSwimSpeed`))
  (bind _linetraceright (`self.LineTraceRight`))
  (bind _linetraceleft (`self.LineTraceLeft`))
  (bind _distanceright (`self.DistanceRight`))
  (bind _distanceleft (`self.DistanceLeft`))
  (bind _skeletalmesh (`self.SkeletalMesh`))
  (bind _skeletalmesh_2 (`self.SkeletalMesh`))
  (bind _camyaw (`self.CamYaw`))
  (bind _skeletalmesh_3 (`self.SkeletalMesh`))
  (bind _returnvalue (`SceneComponent.K2_GetComponentLocation` (`self.LineTraceStart`)))
  (bind _returnvalue_2 (`SceneComponent.K2_GetComponentLocation` (`self.LineTraceStart`)))
  (bind (_returnvalue_x _returnvalue_y) (`KismetMathLibrary.BreakVector` (`SceneComponent.GetForwardVector` _linetraceleft)))
  (bind _returnvalue_3 (`SceneComponent.K2_GetComponentLocation` _linetraceright))
  (bind _returnvalue_4 (`SceneComponent.K2_GetComponentLocation` _linetraceleft))
  (bind (_returnvalue_x_2 _returnvalue_y_2) (`KismetMathLibrary.BreakVector` (`SceneComponent.GetForwardVector` _linetraceright)))
  (bind (_relativerotation_roll _relativerotation_pitch _relativerotation_yaw) (`KismetMathLibrary.BreakRotator` (`SceneComponent.RelativeRotation` _skeletalmesh)))
  (bind (_relativerotation_roll_2 _relativerotation_pitch_2 _relativerotation_yaw_2) (`KismetMathLibrary.BreakRotator` (`SceneComponent.RelativeRotation` _skeletalmesh_2)))
  (bind (_relativerotation_roll_3 _relativerotation_pitch_3 _relativerotation_yaw_3) (`KismetMathLibrary.BreakRotator` (`SceneComponent.RelativeRotation` _skeletalmesh_3)))
  (bind (_relativerotation_roll_4 _relativerotation_pitch_4 _relativerotation_yaw_4) (`KismetMathLibrary.BreakRotator` (`SceneComponent.RelativeRotation` (`self.SkeletalMesh`))))
  (bind (_returnvalue_roll _returnvalue_pitch _returnvalue_yaw) (`KismetMathLibrary.BreakRotator` (`KismetMathLibrary.RLerp` (`KismetMathLibrary.MakeRotator` 0.0 0.0 _camyaw) (`KismetMathLibrary.MakeRotator` 0.0 0.0 _relativerotation_yaw_4) 0.025 true)))
  ;[1 1 1] Spring Arm Adjustment
  (bind _output_get (set `SpringArmComponent.TargetArmLength` (`KismetMathLibrary.Lerp` (stale _output_get) (+ (* _currentswimspeed 200.0) (/ 500.0 _currentswimspeed)) 0.01) (`self.SpringArm`)))
  ;[1 1 1] SWIM
  (if (== (`SkeletalMeshComponent.IsPlaying` (`self.SkeletalMesh`)) false)
    (if (`self.Swimming?`)
      (`SkeletalMeshComponent.PlayAnimation` (`self.SkeletalMesh`) "/Game/Animationer/Turtle4/Turtle4_Anim.Turtle4_Anim" false)
      (`KismetSystemLibrary.Delay` 0.4)
      (if (`self.Dashing?`)
        (set `self.CurrentSwimSpeed` (`self.MaxSpeed`))
        (set `self.Dashing?` false)
        (else
          (set `self.CurrentSwimSpeed` (+ (`self.CurrentSwimSpeed`) 1.5))))))
  ;[1 1 1] LERP Cam Pitch
  (set `self.CamPitch` (`KismetMathLibrary.Lerp` (`self.CamPitch`) (- _relativerotation_pitch_4 25.0) 0.01))
  ;[1 1 1] Reset Cam Yaw
  (if (`self.YawBack?`)
    (set `self.CamYaw` _returnvalue_yaw)
    (`|ExecutionSequence`
      (:`then_0`
        (`KismetSystemLibrary.Delay` 1.0)
        (set `self.YawBack?` false :!label _label_2))
      (:`then_1`
        (if (`KismetMathLibrary.NearlyEqual_FloatFloat` _relativerotation_yaw_4 _camyaw 3.0)
          (goto _label_2)
          (else
            _)))))
  (`SceneComponent.K2_SetRelativeRotation` (`self.SpringArm`) (`KismetMathLibrary.MakeRotator` 0.0 (`self.CamPitch`) (`self.CamYaw`)) false false)
  ;[1 1 1] Forward movement
  (bind _output_get_2 (set `self.CurrentSwimSpeed` (`KismetMathLibrary.FClamp` (- (`self.CurrentSwimSpeed`) (`self.SwimDrag`)) (`self.MinSpeed`) (`self.MaxSpeed`))))
  (`SceneComponent.K2_AddWorldOffset` (`self.DefaultSceneRoot`) (* (`SceneComponent.GetForwardVector` (`self.SkeletalMesh`)) _output_get_2) false false)
  ;[1 1 1] Turn Away From Walls
  (if (`self.TurnRight`)
    (set `self.TurnAngle` (`KismetMathLibrary.Lerp` (`self.TurnAngle`) 70.0 0.01))
    (`SceneComponent.K2_SetRelativeRotation` _skeletalmesh_2 (`KismetMathLibrary.RLerp` (`KismetMathLibrary.MakeRotator` _relativerotation_roll_2 _relativerotation_pitch_2 _relativerotation_yaw_2) (`KismetMathLibrary.MakeRotator` _relativerotation_roll_2 _relativerotation_pitch_2 (+ _relativerotation_yaw_2 55.0)) 0.01 true) false false)
    (elif (`self.TurnLeft`)
      (set `self.TurnAngle` (`KismetMathLibrary.Lerp` (`self.TurnAngle`) -70.0 0.01))
      (`SceneComponent.K2_SetRelativeRotation` _skeletalmesh (`KismetMathLibrary.RLerp` (`KismetMathLibrary.MakeRotator` _relativerotation_roll _relativerotation_pitch _relativerotation_yaw) (`KismetMathLibrary.MakeRotator` _relativerotation_roll _relativerotation_pitch (+ _relativerotation_yaw -55.0)) 0.01 true) false false)
      (else
        ;[1 1 1] LERP Roll Angle
        (set `self.TurnAngle` (`KismetMathLibrary.Lerp` (`self.TurnAngle`) (* (`self.GetInputAxisValue`) 70.0) 0.007)))))
  ;[1 1 1] Ground Check
  (bind _outhit (`KismetSystemLibrary.LineTraceSingle` _returnvalue_2 (- _returnvalue_2 (0.0 0.0 10000.0)) "TraceTypeQuery1"))
  (set `self.HeightAboveGround` (`.Distance` (`GameplayStatics.BreakHitResult` _outhit)))
  ;[1 1 1] Roof Check
  (bind _outhit_2 (`KismetSystemLibrary.LineTraceSingle` _returnvalue (- _returnvalue (0.0 0.0 -10000.0)) "TraceTypeQuery1"))
  (set `self.HeightBelowRoof` (`.Distance` (`GameplayStatics.BreakHitResult` _outhit_2)))
  ;[1 1 1] Left & Right Check
  (bind _outhit_3 (`KismetSystemLibrary.LineTraceSingle` _returnvalue_3 (+ _returnvalue_3 (* (`KismetMathLibrary.MakeVector` _returnvalue_x_2 _returnvalue_y_2) 3000.0)) "TraceTypeQuery1"))
  (set `self.DistanceRight` (`.Distance` (`GameplayStatics.BreakHitResult` _outhit_3)))
  (bind _outhit_4 (`KismetSystemLibrary.LineTraceSingle` _returnvalue_4 (+ _returnvalue_4 (* (`KismetMathLibrary.MakeVector` _returnvalue_x _returnvalue_y) 3000.0)) "TraceTypeQuery1"))
  (set `self.DistanceLeft` (`.Distance` (`GameplayStatics.BreakHitResult` _outhit_4)))
  (if (`self.IsBelowMaxHeight`)
    (if (`self.IsAboveMinHeight`)
      (set `self.CorrectionAngle` (`self.PitchAngle`))
      (else
        (set `self.CorrectionAngle` 25.0)))
    (else
      (set `self.CorrectionAngle` -25.0)))
  ;[1 1 1] LERP Pitch Angle
  (set `self.PitchAngle` (`KismetMathLibrary.Lerp` _pitchangle (`KismetMathLibrary.ClampAngle` (+ _pitchangle (* (`self.GetInputAxisValue`) -25.0)) -55.0 55.0) 0.01))
  ;[1 1 1] Height Restrictions Up & Down
  (bind _output_get_3 (set `self.PitchAngle` (`KismetMathLibrary.Lerp` (`self.PitchAngle`) (`self.CorrectionAngle`) 0.01)))
  (`SceneComponent.K2_SetRelativeRotation` _skeletalmesh_3 (`KismetMathLibrary.MakeRotator` (`self.TurnAngle`) _output_get_3 _relativerotation_yaw_3) false false)
  ;[1 1 1] Set Bools
  (if (< (`self.HeightAboveGround`) (`self.MinHeight`))
    (set `self.IsAboveMinHeight` false))
  (if (> (`self.HeightAboveGround`) (`self.MinRecoveryHeight`))
    (set `self.IsAboveMinHeight` true))
  (if (< (`self.HeightBelowRoof`) (`self.MinHeight`))
    (set `self.IsBelowMaxHeight` false))
  (if (> (`self.HeightBelowRoof`) (`self.MinRecoveryHeight`))
    (set `self.IsBelowMaxHeight` true))
  (if (and (and (!= _distanceright 0.0) (or (< _distanceright 500.0) (< _distanceleft 500.0))) (!= _distanceleft 0.0))
    (if (> (`self.DistanceRight`) (`self.DistanceLeft`))
      (set `self.TurnRight` true)
      (elif (> (`self.DistanceLeft`) (`self.DistanceRight`))
        (set `self.TurnLeft` true)))
    (else
      (`KismetSystemLibrary.Delay` 0.5)
      (set `self.TurnRight` false)
      (set `self.TurnLeft` false))))

(event `InputAction|ResetCamYaw`
  (params (Key :type "Key Structure"))
  ;[1 1 1] Reset Cam Yaw
  (:`Pressed`
    (set `self.YawBack?` true)))

(fn `UserConstructionScript`)