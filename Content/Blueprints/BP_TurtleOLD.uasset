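; BP_TurtleOLD is a player-controlled turtle that constantly moves along its local X axis and swims in strokes.
; LookUp and TurnRight axis inputs share one rotation update that adjusts pitch and yaw.
; SwimStroke resets speed to SwimSpeed, gated by a StrokeDuration cooldown.
; Tick decays speed by a fixed per-frame step to a minimum glide, adding actor roll into the forward offset.
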(event `InputAxis|LookUp`
  (params (AxisValue :type "Float (single-precision)"))
  (bind (_returnvalue_roll _returnvalue_pitch _returnvalue_yaw) (`KismetMathLibrary.BreakRotator` (`self.K2_GetActorRotation`)))
  ;[1 1 1] Steering
  (`self.K2_SetActorRelativeRotation` (`KismetMathLibrary.MakeRotator` _returnvalue_roll (+ (/ (* AxisValue -1.0) 3.0) _returnvalue_pitch) (+ (/ (stale `InputAxis|TurnRight` AxisValue) 3.0) _returnvalue_yaw)) :!label _label))

(event `InputAxis|TurnRight`
  (params (AxisValue :type "Float (single-precision)"))
  ;[1 1 1] Steering
  (goto _label))

(event `InputAction|SwimStroke`
  (params (Key :type "Key Structure"))
  (:`Pressed`
    (if (`self.CanStrokeAgain`)
      (set `self.CurrentSwimSpeed` (`self.SwimSpeed`))
      (set `self.CanStrokeAgain` false)
      (`KismetSystemLibrary.Delay` (`self.StrokeDuration`))
      (set `self.CanStrokeAgain` true))))

(event `self.ReceiveTick`
  (params (DeltaSeconds :type "Float (single-precision)"))
  (bind _returnvalue_roll (`KismetMathLibrary.BreakRotator` (`self.K2_GetActorRotation`)))
  (bind _output_get (set `self.CurrentSwimSpeed` (`KismetMathLibrary.FClamp` (- (`self.CurrentSwimSpeed`) 0.025) 1.0 (`self.SwimSpeed`))))
  (bind _returnvalue_x (`KismetMathLibrary.BreakVector` (+ (`KismetMathLibrary.Conv_DoubleToVector` _returnvalue_roll) _output_get)))
  (`self.K2_AddActorLocalOffset` (`KismetMathLibrary.MakeVector` _returnvalue_x)))

(fn `UserConstructionScript`)